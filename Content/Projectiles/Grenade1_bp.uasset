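; Grenade projectile Blueprint that explodes on a fixed fuse shortly after spawning.
; BeginPlay waits two seconds, then spawns an enlarged explosion emitter at the static mesh, fires a RadialForce impulse, plays the explosion sound and destroys the actor.
; Each hit on the static mesh plays a bounce sound at its location, and the file applies no damage.
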(event `self.ReceiveBeginPlay`
  (`KismetSystemLibrary.Delay` 2.0)
  (`GameplayStatics.SpawnEmitterAtLocation` "/Game/MilitaryWeapDark/FX/P_Grenade_Explosion_01.P_Grenade_Explosion_01" (`SceneComponent.K2_GetComponentLocation` (`self.StaticMesh`)) (struct) (2.0 2.0 2.0))
  (`RadialForceComponent.FireImpulse` (`self.RadialForce`))
  (`GameplayStatics.PlaySoundAtLocation` "/Game/MilitaryWeapDark/Sound/RocketLauncher/RocketLauncher_Explosion_Cue.RocketLauncher_Explosion_Cue" (`SceneComponent.K2_GetComponentLocation` (`self.StaticMesh`)) (struct) 1.0 1.0 0.0 null null null null)
  (`self.K2_DestroyActor`))

(event `self.StaticMesh.OnComponentHit`
  (params (HitComponent :type "PrimitiveComponent Object Reference") (OtherActor :type "Actor Object Reference") (OtherComp :type "PrimitiveComponent Object Reference") (NormalImpulse :type "Vector Structure") (Hit :type "HitResult Structure (by ref)"))
  (`GameplayStatics.PlaySoundAtLocation` "/Game/MilitaryWeapDark/Sound/GrenadeLauncher/GrenadeLauncher_Bounce_Cue.GrenadeLauncher_Bounce_Cue" (`SceneComponent.K2_GetComponentLocation` (`self.StaticMesh`)) (struct) 1.0 1.0 0.0 null null null null))

(fn `UserConstructionScript`)